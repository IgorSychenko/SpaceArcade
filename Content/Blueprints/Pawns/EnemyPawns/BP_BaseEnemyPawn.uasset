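; Base enemy pawn that constantly moves forward and steers toward the player's pawn.
; BeginPlay caches the player as BP_PlayerPawn; Tick offsets along local X by FrontalSpeed.
; While that reference is valid and RotationSpeed is nonzero, it yaws by the clamped look-at delta, with asymmetric limits (ten times wider on the negative side).
; A sharper RInterpTo rotation alternative remains disconnected.
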(event EventBeginPlay
  (|CallParentFunction)
  (bind _asbp_player_pawn (Utilities|Casting|CastToBP_PlayerPawn (Game|Player|GetPlayerPawn 0)))
  (Variables|Default|SetPlayerPawn _asbp_player_pawn))

(event Collision|EventActorBeginOverlap
  (params (OtherActor :type Actor%20Object%20Reference)))

(event EventTick
  (params (DeltaSeconds :type Float%20%28single-precision%29))
  (bind _rotationspeed (Variables|Enemy|GetRotationSpeed))
  (|CallParentFunction DeltaSeconds)
  (Transformation|AddActorLocalOffset (Math|Vector|MakeVector (* DeltaSeconds (Variables|Enemy|GetFrontalSpeed)) 0.0 0.0) false false)
  (Variables|Default|GetPlayerPawn
    (:then
      (if (not (== (Variables|Enemy|GetRotationSpeed) 0.0))
        (Transformation|AddActorLocalRotation (Math|Rotator|MakeRotator 0.0 0.0 (* (Math|Float|Clamp(Float) (.yaw (Math|Rotator|Delta(Rotator) (Math|Rotator|FindLookatRotation (Transformation|GetActorLocation) (Transformation|GetActorLocation (Variables|Default|GetPlayerPawn))) (Transformation|GetActorRotation))) (* _rotationspeed -1e+01) _rotationspeed) (Utilities|Time|GetWorldDeltaSeconds))) false false)))
    (:else)))

(fn ConstructionScript)
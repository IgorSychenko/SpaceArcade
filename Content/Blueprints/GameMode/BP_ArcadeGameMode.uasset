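; BP_ArcadeGameMode is the arcade game mode that shows the mouse cursor and handles level-up and game-over screens.
; On game over, it asks GM_Instance whether GamePoints is a new high score, shows either the high-score or game-over widget, then pauses the game.
; EnemySpawnController's level-up event displays a temporary W_LevelUp banner, removed after a short delay.
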(event OnLevelUp(EnemySpawnController)
  (params (NewLevel :type Integer))
  (bind _returnvalue (UserInterface|CreateWidget "/Game/UI/Menus/W_LevelUp.W_LevelUp_C" (Game|GetPlayerController 0)))
  (UserInterface|Viewport|AddtoViewport _returnvalue 0)
  (Utilities|FlowControl|Delay 2.0)
  (Widget|RemovefromParent _returnvalue))

(event Custom|GameOver
  (bind _returnvalue (Game|GetPlayerController 0))
  (bind _asgm_instance (Utilities|Casting|CastToGM_Instance (Game|GetGameInstance)))
  (bind _isnewhiscore (Default|IsNewHiScore _asgm_instance (Variables|Default|GetGamePoints)))
  (if _isnewhiscore
    (bind _returnvalue_2 (UserInterface|CreateWidget "/Game/UI/Menus/W_NewHiScore.W_NewHiScore_C" _returnvalue))
    (UserInterface|Viewport|AddtoViewport _returnvalue_2 0)
    (else
      (bind _returnvalue_3 (UserInterface|CreateWidget "/Game/UI/Menus/W_GameOver.W_GameOver_C" _returnvalue))
      (UserInterface|Viewport|AddtoViewport _returnvalue_3 0)))
  (Game|SetGamePaused true))

(event EventBeginPlay
  (Variables|/Script/Engine.PlayerController|SetbShowMouseCursor (Game|GetPlayerController 0) true)
  (EventDispatchers|AssignOnGameOver (delegate Custom|GameOver)))

(event EventTick
  (params (DeltaSeconds :type Float%20%28single-precision%29)))

(fn ConstructionScript)
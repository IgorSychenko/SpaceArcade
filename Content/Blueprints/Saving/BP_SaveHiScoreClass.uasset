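; BP_SaveHiScoreClass holds high score data, made up of a score list and the last entered name, and provides a function to rank the scores.
; SortArray runs a selection sort, repeatedly moving the highest remaining entry into a new array for descending order.
; It then rebuilds Data with that array, keeping the name.
; Entries scoring zero or below are never picked, so they drop out.
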(fn SortArray
  (while (LocalVariables|GetNeedNextLoop)
    (LocalVariables|SetNeedNextLoop false)
    (LocalVariables|SetMaxValue 0)
    (bind (_array_element _array_index) (Utilities|Array|ForEachLoopwithBreak (.hiscores (Variables|Default|GetData)))
      (:LoopBody
        (if (> (.value _array_element) (LocalVariables|GetMaxValue))
          (LocalVariables|SetMaxValue (.value _array_element))
          (LocalVariables|SetIndexMaxValue _array_index)
          (LocalVariables|SetNeedNextLoop true)))
      (:Completed
        (if (LocalVariables|GetNeedNextLoop)
          (Utilities|Array|Add (LocalVariables|GetSortedArray) (Utilities|Array|Get(acopy) (.hiscores (Variables|Default|GetData)) (LocalVariables|GetIndexMaxValue)))
          (Utilities|Array|RemoveIndex (.hiscores (Variables|Default|GetData)) (LocalVariables|GetIndexMaxValue))))))
  (Variables|Default|SetData (Utilities|Struct|MakeS_Save (.lastentername (Variables|Default|GetData)) (LocalVariables|GetSortedArray))))
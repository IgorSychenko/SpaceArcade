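; GM_Instance keeps a capped high score table and persists it through BP_SaveHiScoreClass in the "HiScrores" slot.
; AddHiScore uses IsNewHiScore to count higher scores, then removes the last entry if the table is full and appends the new one.
; LoadGame calls SortArray on the loaded object before copying its data.
; SaveGame and SortHiScores call it on newly created objects before any HiScores data is assigned.
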(event Custom|LoadGame
  (bind _returnvalue (SaveGame|LoadGamefromSlot "HiScrores"))
  (bind _asbp_save_hi_score_class (Utilities|Casting|CastToBP_SaveHiScoreClass _returnvalue))
  (Default|SortArray _asbp_save_hi_score_class)
  (Variables|Default|SetHiScores (Variables|/Game/Blueprints/Saving/BP_SaveHiScoreClass.BP_SaveHiScoreClass_C|GetData _asbp_save_hi_score_class)))

(event Custom|SaveGame
  (bind _returnvalue (SaveGame|CreateSaveGameObject "/Game/Blueprints/Saving/BP_SaveHiScoreClass.BP_SaveHiScoreClass_C"))
  (bind _asbp_save_hi_score_class (Utilities|Casting|CastToBP_SaveHiScoreClass _returnvalue))
  (Default|SortArray _asbp_save_hi_score_class)
  (Variables|/Game/Blueprints/Saving/BP_SaveHiScoreClass.BP_SaveHiScoreClass_C|SetData _asbp_save_hi_score_class (Variables|Default|GetHiScores))
  (SaveGame|SaveGametoSlot _asbp_save_hi_score_class "HiScrores"))

(fn AddHiScore
  (params (Name :type Text) (Value :type Integer))
  (bind _isnewhiscore (CallFunction|IsNewHiScore Value))
  (if _isnewhiscore
    (if (>= (Utilities|Array|Length (.hiscores (Variables|Default|GetHiScores))) (Variables|Default|GetNumHiScores))
      (Utilities|Array|RemoveIndex (.hiscores (Variables|Default|GetHiScores)) (Utilities|Array|LastIndex (.hiscores (Variables|Default|GetHiScores)))))
    (bind _output_get (LocalVariables|SetScore (Utilities|Struct|MakeS_HiScore Name Value)))
    (Utilities|Array|Add (.hiscores (Variables|Default|GetHiScores)) _output_get)
    (Variables|Default|SetHiScores (Utilities|Struct|MakeS_Save Name (.hiscores (Variables|Default|GetHiScores))))
    (CallFunction|SortHiScores)
    (return)))

(fn IsNewHiScore
  (params (Score :type Integer))
  (for _array_element (.hiscores (Variables|Default|GetHiScores))
    (if (> (.value _array_element) Score)
      (Math|Integer|IncrementInt (LocalVariables|GetNumMoreScores))))
  (return (> (Variables|Default|GetNumHiScores) (LocalVariables|GetNumMoreScores))))

(fn SortHiScores
  (bind _returnvalue (SaveGame|CreateSaveGameObject "/Game/Blueprints/Saving/BP_SaveHiScoreClass.BP_SaveHiScoreClass_C"))
  (bind _asbp_save_hi_score_class (Utilities|Casting|CastToBP_SaveHiScoreClass _returnvalue))
  (Default|SortArray _asbp_save_hi_score_class))